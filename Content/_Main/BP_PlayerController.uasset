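; Player controller for a slingshot game that turns mouse input into aim and throw commands on the possessed BPA_Player_Slingshot pawn.
; On BeginPlay it adds the slingshot Enhanced Input mapping context, shows the cursor and caches the pawn.
; Pressing records the start mouse position, Ongoing updates the current one, and release (completed or canceled) starts the throw.
; Separate actions cancel the throw or quit; the reset action is unwired.
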(event Input|EnhancedActionEvents|EnhancedInputActionIA_Mouse_press
  (params (ActionValue :type Boolean) (ElapsedSeconds :type Float%20%28double-precision%29) (TriggeredSeconds :type Float%20%28double-precision%29) (InputAction :type Input%20Action%20Object%20Reference :default "/Game/_Inputs/IA_Mouse_press.IA_Mouse_press"))
  (bind (_locationx _locationy) (Game|Player|GetMousePosition))
  (bind _slingshot (Variables|Default|GetSlingshot))
  (bind _returnvalue (Math|Vector2D|MakeVector2D _locationx _locationy))
  (:Started
    (Variables|/Game/_Main/BPA_Player_Slingshot.BPA_Player_Slingshot_C|SetStartMousePosition (Variables|Default|GetSlingshot) _returnvalue))
  (:Ongoing
    (Variables|/Game/_Main/BPA_Player_Slingshot.BPA_Player_Slingshot_C|SetCurrentMousePosition (Variables|Default|GetSlingshot) _returnvalue))
  (:Canceled
    (Variables|/Game/_Main/BPA_Player_Slingshot.BPA_Player_Slingshot_C|SetCurrentMousePosition _slingshot _returnvalue :!label _label)
    (Default|StartItemThrow _slingshot))
  (:Completed
    (goto _label)))

(event Input|EnhancedActionEvents|EnhancedInputActionIA_Mouse_cancel
  (params (ActionValue :type Boolean) (ElapsedSeconds :type Float%20%28double-precision%29) (TriggeredSeconds :type Float%20%28double-precision%29) (InputAction :type Input%20Action%20Object%20Reference :default "/Game/_Inputs/IA_Mouse_cancel.IA_Mouse_cancel"))
  (:Started
    (Default|CancelThrow (Variables|Default|GetSlingshot))))

(event Input|EnhancedActionEvents|EnhancedInputActionIA_Mouse_reset
  (params (ActionValue :type Boolean) (ElapsedSeconds :type Float%20%28double-precision%29) (TriggeredSeconds :type Float%20%28double-precision%29) (InputAction :type Input%20Action%20Object%20Reference :default "/Game/_Inputs/IA_Mouse_reset.IA_Mouse_reset")))

(event Input|EnhancedActionEvents|EnhancedInputActionIA_Quit
  (params (ActionValue :type Boolean) (ElapsedSeconds :type Float%20%28double-precision%29) (TriggeredSeconds :type Float%20%28double-precision%29) (InputAction :type Input%20Action%20Object%20Reference :default "/Game/_Inputs/IA_Quit.IA_Quit"))
  (Game|QuitGame 0 "Quit" false))

(event EventBeginPlay
  (bind _self self)
  (bind _returnvalue (PlayerController|LocalPlayerSubsystems|GetEnhancedInputLocalPlayerSubsystem _self))
  (Utilities|IsValid _returnvalue
    (:Is%20Valid
      (Input|AddMappingContext _returnvalue "/Game/_Inputs/IMC_Slingshot.IMC_Slingshot" 0 "(bIgnoreAllPressedKeysUntilRelease=True,bForceImmediately=False,bNotifyUserSettings=False)")
      (Variables|Default|SetbShowMouseCursor true)
      (bind _asbpa_player_slingshot (Utilities|Casting|CastToBPA_Player_Slingshot (Pawn|GetControlledPawn)))
      (Variables|Default|SetSlingshot _asbpa_player_slingshot))))

(event EventTick
  (params (DeltaSeconds :type Float%20%28single-precision%29)))

(fn ConstructionScript)

(fn GetMouseInput)